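; BP_RunningAI is an AI runner for a red light, green light game run by BP_Doll, with a random walk speed set at spawn.
; Tick moves it forward while alive and RedLight is off, gated by the doll's GameStarting flag being false, and disables movement in the winning zone.
; A DoOnce rolls one death chance per red light, triggering a delayed ragdoll, gunshot at the player's location and random blood decal.
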(event EventBeginPlay
  ;[1 1 1] BeginPlay
  ;;[1 1 1] Create a doll ref
  (bind _returnvalue (Actor|GetActorOfClass "/Game/GameCore/Blueprints/Doll/BP_Doll.BP_Doll_C"))
  (Variables|Default|SetDollRef _returnvalue)
  ;;[1 1 1] Set random speed for spawn AI
  (Variables|/Script/Engine.CharacterMovementComponent|SetMaxWalkSpeed (Variables|Character|GetCharacterMovement) (Math|Random|RandomFloatinRange 1e+02 4e+02))
  (bind _asthird_person_character (Utilities|Casting|CastToThirdPersonCharacter (Game|GetPlayerCharacter 0)))
  (Variables|Default|SetThirdPersonCharacterRef _asthird_person_character))

(event EventTick
  (params (DeltaSeconds :type Float%20%28single-precision%29))
  (bind _bloodarray (Variables|Default|GetBloodArray))
  (bind _capsulecomponent (Variables|Collision|GetCapsuleComponent))
  (bind _returnvalue (Math|Vector|GetForwardVector _capsulecomponent))
  ;[1 1 1] If AI in winning zone, dont move
  (if (Variables|Default|GetbInWinningZone)
    (Pawn|Components|CharacterMovement|DisableMovement (Variables|Character|GetCharacterMovement))
    (else
      ;[1 1 1] Check AI dead or win
      (if (not (Variables|Default|GetbDead))
        ;[1 1 1] Check if game has start
        (if (not (Variables|/Game/GameCore/Blueprints/Doll/BP_Doll.BP_Doll_C|GetbGameStarting (Variables|Default|GetDollRef)))
          ;[1 1 1] Check RedLight
          (if (Variables|/Game/GameCore/Blueprints/Doll/BP_Doll.BP_Doll_C|GetbRedLight (Variables|Default|GetDollRef))
            (Utilities|FlowControl|DoOnce false :!label _label
              (:Completed
                ;[1 1 1] Death Chance
                (if (>= (Math|Random|RandomInteger 10) 8)
                  ;[1 1 1] Random delay between deaths
                  (Utilities|FlowControl|Delay (Math|Random|RandomFloatinRange 0.1 2.0))
                  ;[1 1 1] Set AI is dead
                  (Variables|Default|SetbDead true)
                  ;[1 1 1] Ragdoll
                  (Physics|SetSimulatePhysics (Variables|Collision|GetCapsuleComponent) true)
                  ;[1 1 1] Play gun shot sound
                  (Audio|PlaySoundatLocation "/Game/GameCore/Materials/sounds/gunshot_sound.gunshot_sound" (Transformation|GetWorldLocation (Variables|/Script/Engine.Character|GetMesh (Variables|Default|GetThirdPersonCharacterRef))) "0, 0, 0" 0.5 1.0 0.0 0 0 0)
                  ;[1 1 1] Spawn blood decals
                  (Rendering|Decal|SpawnDecalatLocation (Utilities|Array|Get(acopy) _bloodarray (Math|Random|RandomInteger (Utilities|Array|Length _bloodarray))) "50.000000,50.000000,50.000000" (+ (Transformation|GetWorldLocation (Variables|Character|GetMesh)) (Math|Vector|MakeVector (Math|Random|RandomFloatinRange 0.0 1e+02) (Math|Random|RandomFloatinRange 0.0 1e+02) 0.0)) "-90.000000,0.000000,0.000000" 2e+01))))
            (else
              (Utilities|FlowControl|Sequence ; Reset DoOnce so un-deadAI would still be in the game
                (:then_0
                  (goto _label Reset))
                (:then_1
                  ;[1 1 1] Move forward at current speed
                  (Pawn|Input|AddMovementInput _returnvalue (Math|Vector|VectorLength _returnvalue) false))))))))))

(fn ConstructionScript)