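; BP_Doll is a "Red Light, Green Light" doll that periodically turns its head.
; Tick drives a Delay of random 2 to 6 seconds, which acts as a repeating timer that calls Rotate180.
; Rotate180 uses a FlipFlop to alternate between red light and green light Timelines, each setting the Head's relative yaw.
; The graph only handles this rotation, with no player detection.
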(event Custom|Rotate180
  (Utilities|FlowControl|FlipFlop
    (:A
      ;[1 1 1] Rotate head over time
      (bind _rotation (Timeline|RedLightRotationSpeed PlayFromStart)
        (:Update
          (Transformation|SetRelativeRotation (Variables|Default|GetHead) (Math|Rotator|MakeRotator 0.0 0.0 _rotation) false false))))
    (:B
      (bind _rotation_2 (Timeline|GreenLightRotationSpeed PlayFromStart)
        (:Update
          (Transformation|SetRelativeRotation (Variables|Default|GetHead) (Math|Rotator|MakeRotator 0.0 0.0 _rotation_2) false false))))))

(event EventTick
  (params (DeltaSeconds :type Float%20%28single-precision%29))
  ;[1 1 1] Head rotation
  (Utilities|FlowControl|Delay (Math|Random|RandomFloatinRange 2.0 6.0))
  (CallFunction|Rotate180))

(fn ConstructionScript)