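; BP_EndGameVolume is a trigger volume marking the winning zone that ends the game when the player enters it.
; BeginPlay casts player character 0 to ThirdPersonCharacter and caches the reference.
; When that character begins overlapping EndGameCollision, it sets InWinningZone on the character and calls its CompleteGame.
; Ending the overlap clears the InWinningZone flag.
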(event OnComponentBeginOverlap(EndGameCollision)
  (params (OverlappedComponent :type Primitive%20Component%20Object%20Reference) (OtherActor :type Actor%20Object%20Reference) (OtherComp :type Primitive%20Component%20Object%20Reference) (OtherBodyIndex :type Integer) (bFromSweep :type Boolean) (SweepResult :type Hit%20Result%20Structure%20%28by%20ref%29))
  (bind _thirdpersoncharacterref (Variables|Default|GetThirdPersonCharacterRef))
  ;[1 1 1] Complete the game when player is in winning zone
  (if (== OtherActor _thirdpersoncharacterref)
    (Variables|/Game/GameCore/Blueprints/Characters/ThirdPersonCharacter.ThirdPersonCharacter_C|SetbInWinningZone _thirdpersoncharacterref true)
    (Default|CompleteGame _thirdpersoncharacterref)))

(event OnComponentEndOverlap(EndGameCollision)
  (params (OverlappedComponent :type Primitive%20Component%20Object%20Reference) (OtherActor :type Actor%20Object%20Reference) (OtherComp :type Primitive%20Component%20Object%20Reference) (OtherBodyIndex :type Integer))
  (bind _thirdpersoncharacterref (Variables|Default|GetThirdPersonCharacterRef))
  (if (== OtherActor _thirdpersoncharacterref)
    (Variables|/Game/GameCore/Blueprints/Characters/ThirdPersonCharacter.ThirdPersonCharacter_C|SetbInWinningZone _thirdpersoncharacterref false)))

(event EventBeginPlay
  ;[1 1 1] BeginPlay (set ref to character for BP to use
  (bind _asthird_person_character (Utilities|Casting|CastToThirdPersonCharacter (Game|GetPlayerCharacter 0)))
  (Variables|Default|SetThirdPersonCharacterRef _asthird_person_character))

(fn ConstructionScript)