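; BP_EndGameVolumeAI is an end-game volume that tracks whether the running AI is inside the winning zone, where it is meant to stop moving.
; On BeginPlay it caches a BP_RunningAI reference by casting player character 0.
; EndGameCollision begin and end overlaps set that character's InWinningZone flag true or false, ignoring all other actors.
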(event OnComponentBeginOverlap(EndGameCollision)
  (params (OverlappedComponent :type Primitive%20Component%20Object%20Reference) (OtherActor :type Actor%20Object%20Reference) (OtherComp :type Primitive%20Component%20Object%20Reference) (OtherBodyIndex :type Integer) (bFromSweep :type Boolean) (SweepResult :type Hit%20Result%20Structure%20%28by%20ref%29))
  (bind _airef (Variables|Default|GetAIRef))
  ;[1 1 1] When AI make winning zone, they wont move
  (if (== OtherActor _airef)
    (Variables|/Game/GameCore/Blueprints/Characters/BP_RunningAI.BP_RunningAI_C|SetbInWinningZone _airef true)))

(event OnComponentEndOverlap(EndGameCollision)
  (params (OverlappedComponent :type Primitive%20Component%20Object%20Reference) (OtherActor :type Actor%20Object%20Reference) (OtherComp :type Primitive%20Component%20Object%20Reference) (OtherBodyIndex :type Integer))
  (bind _airef (Variables|Default|GetAIRef))
  (if (== OtherActor _airef)
    (Variables|/Game/GameCore/Blueprints/Characters/BP_RunningAI.BP_RunningAI_C|SetbInWinningZone _airef false)))

(event EventBeginPlay
  ;[1 1 1] BeginPlay (set ref to character for BP to use
  (bind _asbp_running_ai (Utilities|Casting|CastToBP_RunningAI (Game|GetPlayerCharacter 0)))
  (Variables|Default|SetAIRef _asbp_running_ai))

(fn ConstructionScript)